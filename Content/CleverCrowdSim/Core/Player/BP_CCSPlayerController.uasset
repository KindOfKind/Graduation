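; Player controller for the crowd simulation that drives a camera pawn and provides flowfield debug tools.
; Enhanced Input actions move, rotate and zoom the pawn, with the cursor shown in game-and-UI mode.
; A toggle flips debug mode on the game state, letting left and right clicks draw flowfield cost or direction grids around the cursor hit.
; The O key draws averaged crowd group areas regardless of debug mode.
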(event `self.ReceiveBeginPlay`
  (bind _asbp_ccsplayer_pawn (cast `/Game/CleverCrowdSim/Core/Player/BP_CCSPlayerPawn` (`self.K2_GetPawn`))
    (:`then`
      (set `self.PlayerPawn` _asbp_ccsplayer_pawn)
      (bind _asbp_ccsgame_mode (cast `/Game/CleverCrowdSim/Core/GameManagement/BP_CCSGameMode` (`GameplayStatics.GetGameMode`)))
      (set `self.BPGameMode` _asbp_ccsgame_mode)
      (bind _asbp_ccsgame_state (cast `/Game/CleverCrowdSim/Core/GameManagement/BP_CCSGameState` (`GameplayStatics.GetGameState`)))
      (set `self.CCSGameState` _asbp_ccsgame_state)
      (`EnhancedInputSubsystemInterface.AddMappingContext` (subsystem `EnhancedInputLocalPlayerSubsystem`) "/Game/CleverCrowdSim/Inputs/IMC_PlayerPawn.IMC_PlayerPawn" 0 (struct))
      (`WidgetBlueprintLibrary.SetInputMode_GameAndUIEx` self null "DoNotLock" false)
      (set `self.bShowMouseCursor` true))
    (:`CastFailed`
      (`KismetSystemLibrary.PrintString` "Player pawn cast failed!"))))

(event `self.ReceiveTick`
  (params (DeltaSeconds :type "Float (single-precision)"))
  (`self.ShowInfoInDebugModeTick`))

(event `EnhancedInput|/Game/CleverCrowdSim/Inputs/InputActions/Navigation/IA_MoveCamera`
  (params (ActionValue :type "Vector2D Structure") (ElapsedSeconds :type "Float (double-precision)") (TriggeredSeconds :type "Float (double-precision)") (InputAction :type "InputAction Object Reference" :default "/Game/CleverCrowdSim/Inputs/InputActions/Navigation/IA_MoveCamera.IA_MoveCamera"))
  (bind (_x _y) (`KismetMathLibrary.BreakVector2D` ActionValue))
  ;[0.1052 0.1052 0.1052] Camera
  (:`Triggered`
    (`Pawn.AddMovementInput` (`self.PlayerPawn`) (`KismetMathLibrary.GreaterGreater_VectorRotator` (`KismetMathLibrary.Normal` (`KismetMathLibrary.MakeVector` _x _y)) (`self.K2_GetActorRotation` (`self.PlayerPawn`))) 1.0 false)))

(event `EnhancedInput|/Game/CleverCrowdSim/Inputs/InputActions/Navigation/IA_RotateCamera`
  (params (ActionValue :type "Float (double-precision)") (ElapsedSeconds :type "Float (double-precision)") (TriggeredSeconds :type "Float (double-precision)") (InputAction :type "InputAction Object Reference" :default "/Game/CleverCrowdSim/Inputs/InputActions/Navigation/IA_RotateCamera.IA_RotateCamera"))
  ;[0.1052 0.1052 0.1052] Camera
  (:`Triggered`
    (`/Game/CleverCrowdSim/Core/Player/BP_CCSPlayerPawn.RotateCamera` (`self.PlayerPawn`) ActionValue)))

(event `EnhancedInput|/Game/CleverCrowdSim/Inputs/InputActions/Navigation/IA_ZoomCamera`
  (params (ActionValue :type "Float (double-precision)") (ElapsedSeconds :type "Float (double-precision)") (TriggeredSeconds :type "Float (double-precision)") (InputAction :type "InputAction Object Reference" :default "/Game/CleverCrowdSim/Inputs/InputActions/Navigation/IA_ZoomCamera.IA_ZoomCamera"))
  ;[0.1052 0.1052 0.1052] Camera
  (:`Triggered`
    (`/Game/CleverCrowdSim/Core/Player/BP_CCSPlayerPawn.ZoomCamera` (`self.PlayerPawn`) (* ActionValue -1.0))))

(event `EnhancedInput|/Game/CleverCrowdSim/Inputs/InputActions/MainActions/IA_MainClick`
  (params (ActionValue :type Boolean) (ElapsedSeconds :type "Float (double-precision)") (TriggeredSeconds :type "Float (double-precision)") (InputAction :type "InputAction Object Reference" :default "/Game/CleverCrowdSim/Inputs/InputActions/MainActions/IA_MainClick.IA_MainClick"))
  ;[0.1052 0.1052 0.1052] Clicks
  (:`Triggered`
    (if (`CCSGameState.IsDebugMode` (`self.CCSGameState`))
      (`self.DrawGridDebugUnderCursor` true))))

(event `EnhancedInput|/Game/CleverCrowdSim/Inputs/InputActions/MainActions/IA_SecondaryClick`
  (params (ActionValue :type Boolean) (ElapsedSeconds :type "Float (double-precision)") (TriggeredSeconds :type "Float (double-precision)") (InputAction :type "InputAction Object Reference" :default "/Game/CleverCrowdSim/Inputs/InputActions/MainActions/IA_SecondaryClick.IA_SecondaryClick"))
  ;[0.1052 0.1052 0.1052] Clicks
  (:`Triggered`
    (if (`CCSGameState.IsDebugMode` (`self.CCSGameState`))
      (`self.DrawGridDebugUnderCursor` false true))))

(event `EnhancedInput|/Game/CleverCrowdSim/Inputs/InputActions/Debug/IA_ToggleDebugMode`
  (params (ActionValue :type Boolean) (ElapsedSeconds :type "Float (double-precision)") (TriggeredSeconds :type "Float (double-precision)") (InputAction :type "InputAction Object Reference" :default "/Game/CleverCrowdSim/Inputs/InputActions/Debug/IA_ToggleDebugMode.IA_ToggleDebugMode"))
  ;[0.1052 0.1052 0.1052] Debug
  (:`Started`
    (`self.ToggleDebugMode`)))

(event `Key|O`
  (params (Key :type "Key Structure"))
  ;[0.1052 0.1052 0.1052] Debug
  (:`Pressed`
    (`self.DebugDrawCrowdGroupAreasAveraged`)))

(fn `DrawGridDebugUnderCursor`
  (params (bCostsGrid :type Boolean) (bDirectionsGrid :type Boolean))
  (locals (bDrawCostsGrid_LOCAL :type Boolean) (bDrawDirectionsGrid_LOCAL :type Boolean) (CursorHitLocation_LOCAL :type "Vector Structure" :default (0.0 0.0 0.0)))
  (bind (_hitresult _returnvalue) (`self.GetHitResultUnderCursorByChannel` "TraceTypeQuery1"))
  (set `local.bDrawCostsGrid_LOCAL` bCostsGrid)
  (set `local.bDrawDirectionsGrid_LOCAL` bDirectionsGrid)
  (if _returnvalue
    (set `local.CursorHitLocation_LOCAL` (`.Location` (`GameplayStatics.BreakHitResult` _hitresult)))
    (`|ExecutionSequence`
      (:`then_0`
        (if (`local.bDrawCostsGrid_LOCAL`)
          (`FlowfieldDebugBPFunctionLibrary.DrawDebugCostsGridInRadius` (`CCSGameMode.GetFlowfield` (`self.BPGameMode`)) (`local.CursorHitLocation_LOCAL`) 1000.0 0.0)
          (`KismetSystemLibrary.PrintString` "DRAW COSTS GRID DEBUG" true true (struct :`G` 0.66 :`B` 1.0 :`A` 1.0) 0.0)))
      (:`then_1`
        (if (`local.bDrawDirectionsGrid_LOCAL`)
          (`FlowfieldDebugBPFunctionLibrary.DrawDebugDirectionsGridInRadius` (`CCSGameMode.GetFlowfield` (`self.BPGameMode`)) 0 true (`local.CursorHitLocation_LOCAL`) 1000.0 0.0)
          (`KismetSystemLibrary.PrintString` "DRAW DIRECTIONS GRID DEBUG" true true (struct :`G` 0.66 :`B` 1.0 :`A` 1.0) 0.0))))))

(fn `ShowInfoInDebugModeTick`
  (if (`CCSGameState.IsDebugMode` (`self.CCSGameState`))
    (`KismetSystemLibrary.PrintString` "Debug Mode Enabled" true false (struct :`G` 1.0 :`B` 0.427829 :`A` 1.0) 0.0)))

(fn `ToggleDebugMode`
  (`CCSGameState.SetDebugModeEnabled` (`self.CCSGameState`) (not (`CCSGameState.IsDebugMode` (`self.CCSGameState`)))))

(fn `UserConstructionScript`)