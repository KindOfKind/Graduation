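; Player camera pawn for CleverCrowdSim that provides zoom and rotation functions for a spring-arm view.
; ZoomCamera steps the spring arm length by a multiplier and clamps it to the configured zoom range.
; RotateCamera yaws the whole pawn in world space, scaled by speed and frame time, with a clamp on each call's rotation.
; The event graph and construction script are empty, with no input binding or Tick logic.
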(fn `RotateCamera`
  (params (RotationMult :type "Float (double-precision)"))
  (`self.K2_AddActorWorldRotation` (`KismetMathLibrary.MakeRotator` 0.0 0.0 (`KismetMathLibrary.FClamp` (* (* RotationMult (`GameplayStatics.GetWorldDeltaSeconds`)) (`self.CameraRotationSpeed`)) -2.0 2.0))))

(fn `UserConstructionScript`)

(fn `ZoomCamera`
  (params (ZoomMult :type "Float (double-precision)"))
  (bind _camerazoomrange (`self.CameraZoomRange`))
  (set `SpringArmComponent.TargetArmLength` (`KismetMathLibrary.FClamp` (+ (`SpringArmComponent.TargetArmLength` (`self.SpringArm`)) (* ZoomMult (`self.CameraZoomStep`))) (`.Value` (break `FloatRangeBound` (break `FloatRange` _camerazoomrange))) (`.Value` (break `FloatRangeBound` (`.UpperBound` (break `FloatRange` _camerazoomrange))))) (`self.SpringArm`)))