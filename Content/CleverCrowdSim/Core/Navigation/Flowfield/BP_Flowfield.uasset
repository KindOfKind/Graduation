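; BP_Flowfield is a flowfield navigation actor for the crowd simulation; the logic shown here handles only the debug display of its grid area.
; DebugTick toggles the debug visualization component and scales its X and Y to the size calculated from GridSettings.
; It runs every Tick from the cached game state's debug mode, and in the construction script via DrawDebugOnConstruct for an editor preview.
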(event `self.ReceiveBeginPlay`
  (bind _asbp_ccsgame_state (cast `/Game/CleverCrowdSim/Core/GameManagement/BP_CCSGameState` (`GameplayStatics.GetGameState`)))
  (set `self.CCSGameState` _asbp_ccsgame_state))

(event `self.ReceiveTick`
  (params (DeltaSeconds :type "Float (single-precision)"))
  (`self.DebugTick` (`CCSGameState.IsDebugMode` (`self.CCSGameState`))))

(fn `DebugTick`
  (params (bShowDebug :type Boolean))
  (bind (_gridsettings_cellsize _gridsettings_gridsizes) (break `FlowfieldGridSettings` (`self.GridSettings`)))
  (`SceneComponent.SetVisibility` (`self.DebugVisualizationOrigin`) bShowDebug true)
  (if bShowDebug
    (bind _returnvalue (`FlowfieldBPFunctionLibrary.CalculateGridSize` _gridsettings_gridsizes (`KismetMathLibrary.Conv_IntToDouble` _gridsettings_cellsize)))
    (bind (_x _y) (`KismetMathLibrary.BreakVector2D` _returnvalue))
    (`SceneComponent.SetWorldScale3D` (`self.DebugVisualizationOrigin`) (`KismetMathLibrary.MakeVector` (/ _x 100.0) (/ _y 100.0) 1.0))))

(fn `UserConstructionScript`
  (`self.DebugTick` (`self.bDrawDebugOnConstruct`)))